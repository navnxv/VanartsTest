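; Actor that travels along the spline of a referenced Route actor, snapping to its first point in the construction script.
; Each Tick it advances a stored distance by Speed, unscaled by delta time, and sets location and rotation from the spline.
; Closed-loop splines wrap the distance back to zero at the end, while open splines ping-pong between the ends by flipping IsOpposite.
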(event EventTick
  (params (DeltaSeconds :type Float%20%28single-precision%29))
  (bind _route (Variables|Default|GetRoute)
    (:then
      (if (Class|SplineComponent|IsClosedLoop (Variables|/Game/Blueprints/AI/BP_PatrolRoute.BP_PatrolRoute_C|GetSpline _route))
        (CallFunction|ClosedLoopMovement)
        (else
          (CallFunction|EndtoEndMovement))))
    (:else)))

(fn ConstructionScript
  (bind _route (Variables|Default|GetRoute)
    (:then
      (Transformation|SetActorLocationAndRotation (.location (Spline|GetTransformatSplinePoint (Variables|/Game/Blueprints/AI/BP_PatrolRoute.BP_PatrolRoute_C|GetSpline _route) 0 "World" false)) (.rotation (Spline|GetTransformatSplinePoint (Variables|/Game/Blueprints/AI/BP_PatrolRoute.BP_PatrolRoute_C|GetSpline _route) 0 "World" false))))
    (:else)))

(fn EndtoEndMovement
  (bind _speed (Variables|Default|GetSpeed))
  (bind _route (Variables|Default|GetRoute)
    (:then
      (Variables|Default|SetCurrentDistance (+ (Variables|Default|GetCurrentDistance) (select (Variables|Default|GetIsOpposite) (* _speed -1.0) _speed)))
      (Transformation|SetActorLocationAndRotation (.location (Spline|GetTransformatDistanceAlongSpline (Variables|/Game/Blueprints/AI/BP_PatrolRoute.BP_PatrolRoute_C|GetSpline _route) (Variables|Default|GetCurrentDistance) "World" false)) (.rotation (Spline|GetTransformatDistanceAlongSpline (Variables|/Game/Blueprints/AI/BP_PatrolRoute.BP_PatrolRoute_C|GetSpline _route) (Variables|Default|GetCurrentDistance) "World" false)))
      (if (not (Variables|Default|GetIsOpposite))
        (if (>= (Variables|Default|GetCurrentDistance) (Spline|GetSplineLength (Variables|/Game/Blueprints/AI/BP_PatrolRoute.BP_PatrolRoute_C|GetSpline (Variables|Default|GetRoute))))
          (Variables|Default|SetIsOpposite true))
        (elif (<= (Variables|Default|GetCurrentDistance) 0.0)
          (Variables|Default|SetIsOpposite false))))
    (:else)))

(fn ClosedLoopMovement
  (bind _route (Variables|Default|GetRoute)
    (:then
      (Variables|Default|SetCurrentDistance (+ (Variables|Default|GetCurrentDistance) (Variables|Default|GetSpeed)))
      (Transformation|SetActorLocationAndRotation (.location (Spline|GetTransformatDistanceAlongSpline (Variables|/Game/Blueprints/AI/BP_PatrolRoute.BP_PatrolRoute_C|GetSpline _route) (Variables|Default|GetCurrentDistance) "World" false)) (.rotation (Spline|GetTransformatDistanceAlongSpline (Variables|/Game/Blueprints/AI/BP_PatrolRoute.BP_PatrolRoute_C|GetSpline _route) (Variables|Default|GetCurrentDistance) "World" false)))
      (if (>= (Variables|Default|GetCurrentDistance) (Spline|GetSplineLength (Variables|/Game/Blueprints/AI/BP_PatrolRoute.BP_PatrolRoute_C|GetSpline (Variables|Default|GetRoute))))
        (Variables|Default|SetCurrentDistance 0.0)))
    (:else)))