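; Interactable door actor that swings its static mesh open and closed between zero and 90 degrees.
; BeginPlay scales the rotation timeline's play rate from a time-to-open variable in seconds.
; Each Interact event alternates through a FlipFlop between playing the timeline forward and in reverse, and is ignored while it is playing.
; The timeline's alpha drives a rotator lerp on the mesh's relative rotation.
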(event EventInteract
  ;[0.15 0.15 0.15 0.5] Only Happening once you press a key
  (if (not (Audio|Components|Audio|IsPlaying (Variables|Default|GetRotateDoorTimeline)))
    (Utilities|FlowControl|FlipFlop
      (:A
        (bind _alpha (Timeline|RotateDoorTimeline PlayFromStart)
          (:Update
            (Transformation|SetRelativeRotation (Variables|Default|GetStaticMesh) (Math|Rotator|Lerp(Rotator) "0, 0, 0" "0.000000,90.000000,0.000000" _alpha) false false))))
      (:B
        (Timeline|RotateDoorTimeline ReverseFromEnd)))))

(event EventBeginPlay
  (Components|Timeline|SetPlayRate (Variables|Default|GetRotateDoorTimeline) (/ 1.0 (Variables|Default|GetTimeToOpenDoor%28InSeconds%29))))

(fn ConstructionScript)