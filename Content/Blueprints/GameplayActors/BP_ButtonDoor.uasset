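; BP_ButtonDoor is a door actor that toggles between closed and raised each time its Trigger event fires.
; Trigger flips the Open flag, playing a Timeline to open or reversing it from the end to close.
; The Timeline lerps the static mesh's relative height.
; The construction script matches mesh and Timeline position to Open, so the door can start in either state.
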(event EventTrigger
  (params (Enable? :type Boolean))
  (bind _output_get (Variables|Default|SetOpen? (not (Variables|Default|GetOpen?))))
  (if _output_get
    (bind _newtrack_0 (Timeline|Timeline Play)
      (:Update
        (Transformation|SetRelativeLocation (Variables|Default|GetStaticMesh) (Math|Vector|Lerp(Vector) "0, 0, 0" "0.000000,0.000000,300.000000" _newtrack_0) false false)))
    (else
      (Timeline|Timeline ReverseFromEnd))))

(fn ConstructionScript
  (bind _timeline (Variables|Default|GetTimeline))
  (if (Variables|Default|GetOpen?)
    (Transformation|SetRelativeLocation (Variables|Default|GetStaticMesh) "0.000000,0.000000,300.000000" false false)
    (Components|Timeline|SetPlaybackPosition _timeline (Components|Timeline|GetTimelineLength _timeline) false true)
    (else
      (Transformation|SetRelativeLocation (Variables|Default|GetStaticMesh) "0, 0, 0" false false)
      (Components|Timeline|SetPlaybackPosition (Variables|Default|GetTimeline) 0.0 false true))))