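; BP_Button is an interactable push button that sends trigger messages to other actors.
; Each Interact flips Enabled and plays or reverses a timeline that slides the Cylinder vertically between pressed and raised positions.
; It then sends every valid actor in ActorsToTriggerMap its own mapped value, independent of Enabled.
; An array-based ManageActorsToTrigger event, which would send Enabled, exists but is not called here.
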(event Custom|ManageActorsToTrigger
  (for _array_element (Variables|Default|GetActorsToTrigger)
    (Utilities|IsValid _array_element
      (:Is%20Valid
        (Class|BPITrigger|Trigger(Message) _array_element (Variables|Default|GetEnabled?))))))

(event Custom|ManageActorsToTriggerMap
  (bind _keys (Utilities|Map|Keys (Variables|Default|GetActorsToTriggerMap)))
  (for _array_element _keys
    (Utilities|IsValid _array_element
      (:Is%20Valid
        (Class|BPITrigger|Trigger(Message) _array_element (.Value (Utilities|Map|Find (Variables|Default|GetActorsToTriggerMap) _array_element)))))))

(event EventBeginPlay)

(event Collision|EventActorBeginOverlap
  (params (OtherActor :type Actor%20Object%20Reference)))

(event EventTick
  (params (DeltaSeconds :type Float%20%28single-precision%29)))

(event EventInteract
  (bind _isa (Utilities|FlowControl|FlipFlop)
    (:A
      (Variables|Default|SetEnabled? _isa)
      (CallFunction|ManageActorstoTriggerMap)
      (bind _alpha (Timeline|ButtonMovingTimeline Play)
        (:Update
          (Transformation|SetRelativeLocation (Variables|Default|GetCylinder) (Math|Vector|Lerp(Vector) "0.000000,0.000000,10.000000" "0.000000,0.000000,-10.000000" _alpha) false false))))
    (:B
      (Variables|Default|SetEnabled? _isa)
      (CallFunction|ManageActorstoTriggerMap)
      (Timeline|ButtonMovingTimeline Reverse))))

(fn ConstructionScript)