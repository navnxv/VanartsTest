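; Base weapon Blueprint that handles semi-auto and automatic firing, with a looping timer repeating shots for automatic fire.
; Each shot traces from the camera, pushed forward by the spring arm length, adding random spread when hip firing.
; The hit either drives hitscan point damage, surface-specific Niagara impacts and a muzzle flash, or aims a projectile spawned at the muzzle socket toward the traced point.
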(event Custom|TryShoot
  (params (TargetArmLength :type Float%20%28double-precision%29))
  (switch Utilities|FlowControl|Switch|SwitchonE_WeaponType (Variables|Default|GetWeaponType)
    (:NewEnumerator0
      (CallFunction|Shoot TargetArmLength))
    (:NewEnumerator1
      (bind _returnvalue (Utilities|Time|SetTimerbyEvent (delegate Custom|TimerShoot) (Variables|Default|GetInterval) true))
      (Variables|Default|SetShootingTimer _returnvalue)
      (CallFunction|Shoot TargetArmLength))))

(event Custom|Shoot
  (params (TargetArmLength :type Float%20%28double-precision%29))
  (bind _returnvalue (Game|GetPlayerCameraManager 0))
  (bind _returnvalue_2 (Transformation|GetActorLocation _returnvalue))
  (bind _returnvalue_3 (Transformation|GetActorForwardVector _returnvalue))
  (bind _returnvalue_4 (* _returnvalue_3 TargetArmLength))
  (bind _returnvalue_5 (+ _returnvalue_2 _returnvalue_4))
  (bind (_outhit _returnvalue_6) (Collision|LineTraceByChannel _returnvalue_5 (+ _returnvalue_5 (* (CallFunction|GetShootDirection (Variables|Default|GetIsPlayerAiming?)) 5e+08)) "TraceTypeQuery1" false 0 "ForOneFrame"))
  (if (Variables|Default|GetUseProjectile?)
    (CallFunction|ProjectileShooting _outhit)
    (else
      (CallFunction|LineTraceShooting _outhit _returnvalue_6))))

(event Custom|TimerShoot
  (CallFunction|Shoot (stale Custom|TryShoot TargetArmLength)))

(event Custom|StopShooting
  (switch Utilities|FlowControl|Switch|SwitchonE_WeaponType (Variables|Default|GetWeaponType)
    (:NewEnumerator1
      (Utilities|Time|ClearandInvalidateTimerbyHandle (Variables|Default|GetShootingTimer)))))

(fn ConstructionScript)

(fn GetShootDirection
  (params (IsAiming? :type Boolean))
  (bind _returnvalue (Game|GetPlayerCameraManager 0))
  (bind _hipfirespread (Variables|Default|GetHipFireSpread))
  (bind _hipfirespread_2 (Variables|Default|GetHipFireSpread))
  (if IsAiming?
    (return (Transformation|GetActorForwardVector (Game|GetPlayerCameraManager 0)))
    (else
      (return (Math|Vector|Normalize (+ (Transformation|GetActorForwardVector _returnvalue) (* (Transformation|GetActorRightVector _returnvalue) (Math|Random|RandomFloatinRange (* _hipfirespread_2 -1.0) _hipfirespread_2)) (* (Transformation|GetActorUpVector _returnvalue) (Math|Random|RandomFloatinRange (* _hipfirespread -1.0) _hipfirespread))))))))

(fn LineTraceShooting
  (params (Hit :type Hit%20Result%20Structure%20%28by%20ref%29) (Hit? :type Boolean))
  (bind (_bblockinghit _binitialoverlap _time _distance _location _impactpoint _normal _impactnormal _physmat) (Collision|BreakHitResult Hit))
  (Utilities|FlowControl|Sequence
    (:then_0
      (if (.bBlockingHit (Collision|BreakHitResult Hit))
        (Utilities|FlowControl|Sequence
          (:then_0
            (Game|Damage|ApplyPointDamage (.HitActor (Collision|BreakHitResult Hit)) (+ (Variables|Default|GetBase%20Damage) (Math|Random|RandomFloatinRange -5.0 5.0)) (Transformation|GetActorLocation) Hit))
          (:then_1
            (Niagara|SpawnSystematLocation (.Value (Utilities|Map|Find (Variables|Default|GetImpactEffects) (Variables|/Script/PhysicsCore.PhysicalMaterial|GetSurfaceType _physmat))) _location (Math|Rotator|MakeRotfromX _normal) "5.000000,5.000000,5.000000" true true "AutoRelease")))))
    (:then_1
      (Niagara|SpawnSystemAttached "/Game/NiagaraExamples/FX_Weapons/MuzzleFlashes/NS_MuzzleFlash.NS_MuzzleFlash" (Variables|Default|GetSkeletalMesh) "Muzzle" "0, 0, 0" "0, 0, 0" "KeepRelativeOffset" true true "AutoRelease"))))

(fn ProjectileShooting
  (params (HitResult :type Hit%20Result%20Structure))
  (bind (_bblockinghit _binitialoverlap _time _distance _location _impactpoint _normal _impactnormal _physmat _hitactor _hitcomponent _hitbonename _bonename _hititem _elementindex _faceindex _tracestart _traceend) (Collision|BreakHitResult HitResult))
  (bind _returnvalue (Game|SpawnActorfromClass "/Game/NiagaraExamples/FX_Weapons/Projectiles/BP_ImpactProjectile.BP_ImpactProjectile_C" (Math|Transform|MakeTransform (Transformation|GetSocketLocation (Variables|Default|GetSkeletalMesh) "Muzzle") (Math|Rotator|FindLookatRotation (Transformation|GetSocketLocation (Variables|Default|GetSkeletalMesh) "Muzzle") (select _bblockinghit _location _traceend)) "1.000000,1.000000,1.000000") "AdjustIfPossibleButAlwaysSpawn" "MultiplyWithRoot" self (Variables|Actor|GetInstigator)))
  (Collision|IgnoreActorwhenMoving (Variables|/Game/NiagaraExamples/FX_Weapons/Projectiles/BP_ProjectileMaster.BP_ProjectileMaster_C|GetCollisionSphere _returnvalue) (Components|GetOwner) true))