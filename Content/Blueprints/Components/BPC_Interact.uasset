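; Actor component on the third-person character that lets the player interact with objects in view.
; A Visibility line trace starts at the camera, pushed forward by the spring arm length, and ignores the owning character.
; Every tick it shows the interact prompt widget only while the hit actor implements BPI_Interact.
; The interaction input repeats the trace and sends InteractMessage to the hit actor.
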(event Input|EnhancedActionEvents|EnhancedInputActionIA_Interaction
  (params (ActionValue :type Boolean) (ElapsedSeconds :type Float%20%28double-precision%29) (TriggeredSeconds :type Float%20%28double-precision%29) (InputAction :type Input%20Action%20Object%20Reference :default "/Game/Input/Actions/IA_Interaction.IA_Interaction"))
  (:Started
    (bind _outhit (CallFunction|TryLineTrace))
    (Class|BPIInteract|Interact(Message) (.HitActor (Collision|BreakHitResult _outhit)))))

(event EventBeginPlay
  (bind _asbp_third_person_character (Utilities|Casting|CastToBP_ThirdPersonCharacter (Components|GetOwner)))
  (Variables|Default|SetPlayerCharacter _asbp_third_person_character)
  (bind _returnvalue (UserInterface|CreateWidget "/Game/Blueprints/UI/WBP_Interact.WBP_Interact_C"))
  (bind _output_get (Variables|Default|SetInteractWidget _returnvalue))
  (UserInterface|Viewport|AddtoViewport _output_get 0)
  (Widget|SetVisibility (Variables|Default|GetInteractWidget) "Collapsed"))

(event EventTick
  (params (DeltaSeconds :type Float%20%28single-precision%29))
  (bind _interactwidget (Variables|Default|GetInteractWidget))
  (bind _outhit (CallFunction|TryLineTrace))
  (if (.bBlockingHit (Collision|BreakHitResult _outhit))
    (if (Utilities|DoesObjectImplementInterface (.HitActor (Collision|BreakHitResult _outhit)) "/Game/Blueprints/Interfaces/BPI_Interact.BPI_Interact_C")
      (Widget|SetVisibility _interactwidget "Visible")
      (else
        (Widget|SetVisibility _interactwidget "Collapsed" :!label _label)))
    (else
      (goto _label))))

(fn TryLineTrace
  (bind _returnvalue (Game|GetPlayerCameraManager 0))
  (bind _playercharacter (Variables|Default|GetPlayerCharacter))
  (bind _returnvalue_2 (Transformation|GetActorLocation _returnvalue))
  (bind _returnvalue_3 (Transformation|GetActorForwardVector _returnvalue))
  (bind _springarm (Variables|/Game/Blueprints/BP_ThirdPersonCharacter.BP_ThirdPersonCharacter_C|GetSpringArm _playercharacter))
  (bind _targetarmlength (Variables|/Script/Engine.SpringArmComponent|GetTargetArmLength _springarm))
  (bind _returnvalue_4 (* _returnvalue_3 _targetarmlength))
  (bind _returnvalue_5 (+ _returnvalue_2 _returnvalue_4))
  (bind _outhit (Collision|LineTraceByChannel _returnvalue_5 (+ _returnvalue_5 (* _returnvalue_3 1e+03)) "TraceTypeQuery1" false (Utilities|Array|MakeArray (Variables|Default|GetPlayerCharacter)) "None" true "(R=1.000000,G=0.000000,B=0.000000,A=1.000000)" "(R=0.000000,G=1.000000,B=0.000000,A=1.000000)" 1.0))
  (return _outhit))