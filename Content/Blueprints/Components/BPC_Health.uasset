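; Health component that tracks its owner's health and signals death when it runs out.
; Health starts at MaxHealth on BeginPlay, and HandleDamageFunction subtracts damage, clamped between zero and the maximum.
; The result goes through SetCurrentHealth, which calls OnDeath whenever the new value is zero or below, with no guard against repeat calls.
; Direct calls to SetCurrentHealth bypass the clamp.
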(event EventBeginPlay
  (Variables|Default|SetHealth (Variables|Default|GetMaxHealth)))

(fn HandleDamageFunction
  (params (Damage :type Float%20%28double-precision%29))
  (CallFunction|SetCurrentHealth (Math|Float|Clamp(Float) (- (Variables|Default|GetHealth) Damage) 0.0 (Variables|Default|GetMaxHealth))))

(fn GetCurrentHealth
  (return (Variables|Default|GetHealth)))

(fn SetCurrentHealth
  (params (NewHealth :type Float%20%28double-precision%29))
  (bind _output_get (Variables|Default|SetHealth NewHealth))
  (if (<= _output_get 0.0)
    (Default|CallOnDeath)))