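; Hazard volume that repeatedly damages third-person characters inside its Box and knocks them back on entry.
; Begin overlap sets the tick interval, enables actor tick and launches the character against its normalized velocity, overriding current motion.
; Each tick applies base damage to every overlapping character, so the tick interval paces the damage.
; Any character's end overlap disables tick, even if others remain inside.
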(event OnComponentBeginOverlap(Box)
  (params (OverlappedComponent :type Primitive%20Component%20Object%20Reference) (OtherActor :type Actor%20Object%20Reference) (OtherComp :type Primitive%20Component%20Object%20Reference) (OtherBodyIndex :type Integer) (bFromSweep :type Boolean) (SweepResult :type Hit%20Result%20Structure%20%28by%20ref%29))
  (bind _asbp_third_person_character (Utilities|Casting|CastToBP_ThirdPersonCharacter OtherActor))
  (Actor|Tick|SetActorTickInterval (Variables|Default|GetTickInterval))
  (Actor|Tick|SetActorTickEnabled true)
  (Character|LaunchCharacter _asbp_third_person_character (* (Math|Vector|Normalize (Transformation|GetVelocity _asbp_third_person_character)) -1.0 1e+03) true true))

(event OnComponentEndOverlap(Box)
  (params (OverlappedComponent :type Primitive%20Component%20Object%20Reference) (OtherActor :type Actor%20Object%20Reference) (OtherComp :type Primitive%20Component%20Object%20Reference) (OtherBodyIndex :type Integer))
  (Utilities|Casting|CastToBP_ThirdPersonCharacter OtherActor)
  (Actor|Tick|SetActorTickEnabled false))

(event EventTick
  (params (DeltaSeconds :type Float%20%28single-precision%29))
  (for _array_element (Collision|GetOverlappingActors (Variables|Default|GetBox) "/Game/Blueprints/BP_ThirdPersonCharacter.BP_ThirdPersonCharacter_C" :!class /Script/Engine.PrimitiveComponent)
    (Game|Damage|ApplyDamage _array_element (Variables|Default|GetBase%20Damage) 0 0)))

(fn ConstructionScript)