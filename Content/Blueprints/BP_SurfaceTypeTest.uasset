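; BP_SurfaceTypeTest is a test actor that represents one surface type, pairing a cube with a text label naming that type.
; The construction script writes the SurfaceType enum's name into the TextRender.
; On BeginPlay it looks up SurfaceType in the PhysicsMats map and applies that physical material as an override on the cube.
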(event EventBeginPlay
  (Class|PrimitiveComponent|SetPhysMaterialOverride (Variables|Default|GetCube) (.Value (Utilities|Map|Find (Variables|Default|GetPhysicsMats) (Variables|Default|GetSurfaceType)))))

(fn ConstructionScript
  (Rendering|Components|TextRender|SetText (Variables|Default|GetTextRender) (Utilities|Text|ToText(String) (Utilities|String|EnumtoString (Variables|Default|GetSurfaceType)))))