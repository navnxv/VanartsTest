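; BP_SimpleNPC is a melee enemy that chases the player and attacks when its DamageSphere overlaps them.
; Overlap pauses the Tick-driven chase and starts a looping timer that plays montages; leaving resumes pursuit.
; A boolean montage map gives random picks without repeats until all are used.
; Attack damages actors in the sphere; incoming point damage feeds the health component, whose death event triggers ragdoll.
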(event OnComponentBeginOverlap(DamageSphere)
  (params (OverlappedComponent :type Primitive%20Component%20Object%20Reference) (OtherActor :type Actor%20Object%20Reference) (OtherComp :type Primitive%20Component%20Object%20Reference) (OtherBodyIndex :type Integer) (bFromSweep :type Boolean) (SweepResult :type Hit%20Result%20Structure%20%28by%20ref%29))
  (if (== OtherActor (Game|GetPlayerCharacter 0))
    (Components|Movement|StopMovementImmediately (Variables|Character|GetCharacterMovement))
    (Actor|Tick|SetActorTickEnabled false)
    (CallFunction|TryActivateMontage)
    (bind _returnvalue (Utilities|Time|SetTimerbyEvent (delegate Custom|TryActivateMontage) 0.2 true))
    (Variables|Default|SetAnimtimer _returnvalue)))

(event OnDeath(BPC_Health)
  (bind _mesh (Variables|Character|GetMesh))
  (Collision|SetCollisionEnabled (Variables|Collision|GetCapsuleComponent) "NoCollision")
  (Physics|SetSimulatePhysics _mesh true)
  (Collision|SetCollisionProfileName _mesh "Ragdoll" true :!class /Script/Engine.PrimitiveComponent))

(event OnComponentEndOverlap(DamageSphere)
  (params (OverlappedComponent :type Primitive%20Component%20Object%20Reference) (OtherActor :type Actor%20Object%20Reference) (OtherComp :type Primitive%20Component%20Object%20Reference) (OtherBodyIndex :type Integer))
  (Animation|Montage|MontageStop (Components|SkeletalMesh|GetAnimInstance (Variables|Character|GetMesh)) 0.0 0)
  (Actor|Tick|SetActorTickEnabled true)
  (Utilities|Time|ClearandInvalidateTimerbyHandle (Variables|Default|GetAnimtimer)))

(event Custom|Attack
  (for _array_element (Collision|GetOverlappingActors (Variables|Default|GetDamageSphere) "/Script/Engine.Actor" :!class /Script/Engine.PrimitiveComponent)
    (Game|Damage|ApplyDamage _array_element 1e+01 (Pawn|GetController) self)))

(event Custom|TryActivateMontage
  (if (not (Animation|Montage|MontageIsPlaying (Components|SkeletalMesh|GetAnimInstance (Variables|Character|GetMesh)) 0))
    (bind _l_chosenanimtion1 (CallFunction|GetMontagetoPlay))
    (bind _output_get (Variables|Default|SetCurrentChosenActiveMontage _l_chosenanimtion1))
    (Animation|Montage|PlayMontage (Variables|Character|GetMesh) _output_get)))

(event EventBeginPlay
  (Variables|Default|SetActiveListOfAttackMontages (Variables|Default|GetAttackMontages)))

(event EventTick
  (params (DeltaSeconds :type Float%20%28single-precision%29))
  (AI|Navigation|SimpleMovetoActor (Pawn|GetController) (Game|GetPlayerCharacter 0)))

(event Game|Damage|EventPointDamage
  (params (Damage :type Float%20%28single-precision%29) (DamageType :type Damage%20Type%20Object%20Reference) (HitLocation :type Vector :default "0, 0, 0") (HitNormal :type Vector :default "0, 0, 0") (HitComponent :type Primitive%20Component%20Object%20Reference) (BoneName :type Name :default "None") (ShotFromDirection :type Vector :default "0, 0, 0") (InstigatedBy :type Controller%20Object%20Reference) (DamageCauser :type Actor%20Object%20Reference) (HitInfo :type Hit%20Result%20Structure%20%28by%20ref%29))
  (Default|HandleDamageFunction (Variables|Default|GetBPC_Health) Damage)
  (Development|PrintString (Utilities|String|ToString(Float) (Default|GetCurrentHealth (Variables|Default|GetBPC_Health)))))

(fn ConstructionScript)

(fn GetMontagetoPlay
  (bind _retrunvalue (CallFunction|CheckifMapHasValidMontage))
  (if _retrunvalue
    _
    (else
      (CallFunction|ResetMap)))
  (bind _keys (Utilities|Map|Keys (Variables|Default|GetMontagesMap) :!label _label))
  (bind _output_get (LocalVariables|SetL_ChosenAnimtion (.OutItem (Utilities|Array|Random _keys))))
  (if (.Value (Utilities|Map|Find (Variables|Default|GetMontagesMap) _output_get))
    (goto _label)
    (else
      (Utilities|Map|Add (Variables|Default|GetMontagesMap) (LocalVariables|GetL_ChosenAnimtion) true)
      (return (LocalVariables|GetL_ChosenAnimtion)))))

(fn CheckifMapHasValidMontage
  (bind _valuepin (Utilities|Map|ForEachLoop(Map) (Variables|Default|GetMontagesMap))
    (:then
      (if (not _valuepin)
        (return true)))
    (:CompletedPin
      (return false))))

(fn ResetMap
  (bind _keypin (Utilities|Map|ForEachLoop(Map) (Variables|Default|GetMontagesMap))
    (:then
      (Utilities|Map|Add (Variables|Default|GetMontagesMap) _keypin false))))