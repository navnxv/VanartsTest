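; BP_NPC is an AI character that lobs grenades at targets, takes damage and ragdolls on death.
; TryAttack spawns BP_Grenade with a predicted launch velocity for a moving target and a randomized flight time; homing nodes exist but are disconnected.
; Damage feeds the health component, whose death event enables ragdoll physics and stops the AI brain logic.
; Capsule hits are reported as touch events for AI perception.
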(event OnComponentBeginOverlap(CapsuleComponent)
  (params (OverlappedComponent :type Primitive%20Component%20Object%20Reference) (OtherActor :type Actor%20Object%20Reference) (OtherComp :type Primitive%20Component%20Object%20Reference) (OtherBodyIndex :type Integer) (bFromSweep :type Boolean) (SweepResult :type Hit%20Result%20Structure%20%28by%20ref%29)))

(event OnComponentHit(CapsuleComponent)
  (params (HitComponent :type Primitive%20Component%20Object%20Reference) (OtherActor :type Actor%20Object%20Reference) (OtherComp :type Primitive%20Component%20Object%20Reference) (NormalImpulse :type Vector :default "0, 0, 0") (Hit :type Hit%20Result%20Structure%20%28by%20ref%29))
  (Class|AISenseTouch|ReportTouchEvent self OtherActor (Transformation|GetActorLocation)))

(event OnDeath(BPC_Health)
  (bind _mesh (Variables|Character|GetMesh))
  (Physics|SetSimulatePhysics _mesh true)
  (Collision|SetCollisionProfileName _mesh "Ragdoll" true :!class /Script/Engine.PrimitiveComponent)
  (Collision|SetCollisionEnabled (Variables|Collision|GetCapsuleComponent) "NoCollision")
  (AI|Logic|StopLogic (Variables|/Script/AIModule.AIController|GetBrainComponent (AI|GetAIController self)) "Dead"))

(event Custom|TryAttack
  (params (TargetActor :type Actor%20Object%20Reference))
  (bind _self self)
  (bind _projectilespawnlocation (Variables|Default|GetProjectileSpawnLocation))
  (bind _returnvalue (Transformation|GetWorldLocation _projectilespawnlocation))
  (bind _outlaunchvelocity (Class|GameplayStatics|SuggestProjectileVelocityMovingTarget (Transformation|GetWorldLocation (Variables|Default|GetProjectileSpawnLocation)) TargetActor "0, 0, 0" 0.0 (Math|Random|RandomFloatinRange 0.5 1.5)))
  (bind _returnvalue_2 (Game|SpawnActorfromClass "/Game/Blueprints/Weapons/BP_Grenade.BP_Grenade_C" (Math|Transform|MakeTransform _returnvalue (Math|Rotator|FindLookatRotation _returnvalue (Transformation|GetActorLocation TargetActor)) "1.000000,1.000000,1.000000") "AdjustIfPossibleButAlwaysSpawn" "MultiplyWithRoot" _self _self))
  (Variables|/Script/Engine.ProjectileMovementComponent|SetMaxSpeed (Variables|/Game/Blueprints/Weapons/BP_Grenade.BP_Grenade_C|GetProjectileMovement _returnvalue_2) (Math|Vector|VectorLength _outlaunchvelocity))
  (Variables|/Script/Engine.MovementComponent|SetVelocity (Variables|/Game/Blueprints/Weapons/BP_Grenade.BP_Grenade_C|GetProjectileMovement _returnvalue_2) _outlaunchvelocity))

(event Game|Damage|EventAnyDamage
  (params (Damage :type Float%20%28single-precision%29) (DamageType :type Damage%20Type%20Object%20Reference) (InstigatedBy :type Controller%20Object%20Reference) (DamageCauser :type Actor%20Object%20Reference))
  (Default|HandleDamageFunction (Variables|Default|GetBPC_Health) Damage))

(fn ConstructionScript)