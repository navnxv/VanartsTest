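; BP_Spawner is a trigger-volume spawner that populates its area while the third-person character is inside its box.
; On overlap begin, it loops over the SpawnParams map of classes to counts, spawning each at randomly chosen actor transforms from Locations.
; Spawned actors are tracked in an array, then destroyed and cleared when the character leaves the box.
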(event OnComponentBeginOverlap(Box)
  (params (OverlappedComponent :type Primitive%20Component%20Object%20Reference) (OtherActor :type Actor%20Object%20Reference) (OtherComp :type Primitive%20Component%20Object%20Reference) (OtherBodyIndex :type Integer) (bFromSweep :type Boolean) (SweepResult :type Hit%20Result%20Structure%20%28by%20ref%29))
  (Utilities|Casting|CastToBP_ThirdPersonCharacter OtherActor)
  (bind _keys (Utilities|Map|Keys (Variables|Default|GetSpawnParams)))
  (for _array_element _keys
    (for _index (range 0 (.Value (Utilities|Map|Find (Variables|Default|GetSpawnParams) _array_element)))
      (bind _returnvalue (Game|SpawnActorfromClass _array_element (Transformation|GetActorTransform (.OutItem (Utilities|Array|Random (Variables|Default|GetLocations)))) "AdjustIfPossibleButAlwaysSpawn" "MultiplyWithRoot" 0 0))
      (Utilities|Array|Add (Variables|Default|GetSpawnedActors) _returnvalue))))

(event OnComponentEndOverlap(Box)
  (params (OverlappedComponent :type Primitive%20Component%20Object%20Reference) (OtherActor :type Actor%20Object%20Reference) (OtherComp :type Primitive%20Component%20Object%20Reference) (OtherBodyIndex :type Integer))
  (Utilities|Casting|CastToBP_ThirdPersonCharacter OtherActor)
  (for _array_element (Variables|Default|GetSpawnedActors)
    (Utilities|IsValid _array_element
      (:Is%20Valid
        (Actor|DestroyActor _array_element))))
  (Utilities|Array|Clear (Variables|Default|GetSpawnedActors)))

(fn ConstructionScript)